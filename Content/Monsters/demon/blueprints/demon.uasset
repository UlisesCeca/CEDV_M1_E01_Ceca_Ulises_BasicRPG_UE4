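; Demon enemy that chases the player's asesina character, attacks in melee, and awards a point on death.
; Pawn sensing drives AIMoveTo, whose results set a nearness flag and the demonABP walk and attack flags.
; Offset looping timers trigger the attack animation when near and damage asesina actors overlapping the melee capsule.
; Incoming damage lowers health, shown on a widget bar every Tick; death flags the AnimBP, then destroys the actor after a delay.
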(event OnSeePawn(sensor)
  (params (Pawn :type Pawn%20Object%20Reference))
  ;[1 1 1] IA seguir
  (bind _asasesina (Utilities|Casting|CastToasesina Pawn))
  (AI|AIMoveTo self "0, 0, 0" _asasesina 1.5e+02 false
    (:OnSuccess
      (Variables|Default|Setcerca true)
      (CallFunction|Noperseguir)
      (CallFunction|NoAtacar))
    (:OnFail
      (Variables|Default|Setcerca false)
      (CallFunction|Perseguir))))

(event EventTick
  (params (DeltaSeconds :type Float%20%28single-precision%29))
  ;[1 1 1] actualizar barra vida
  (bind _asvida_enemigo (Utilities|Casting|CastTovida_enemigo (UserInterface|GetUserWidgetObject (Variables|Default|GetWidget))))
  (Progress|SetPercent (Variables|/Game/misc/vida_enemigo.vida_enemigo_C|GetProgressBar_41 _asvida_enemigo) (/ (Math|Conversions|ToFloat(Integer) (Variables|Default|Gethealth)) 1e+02)))

(event Game|Damage|EventAnyDamage
  (params (Damage :type Float%20%28single-precision%29) (DamageType :type Damage%20Type%20Object%20Reference) (InstigatedBy :type Controller%20Object%20Reference) (DamageCauser :type Actor%20Object%20Reference))
  ;[1 1 1] recibir daño y morir
  (if (Variables|Default|Getalive)
    (Variables|Default|Sethealth (- (Variables|Default|Gethealth) (Math|Float|Floor Damage)))
    (if (<= (Variables|Default|Gethealth) 0)
      (Variables|Default|Setalive false)
      (bind _asdemon_abp (Utilities|Casting|CastTodemonABP (Components|SkeletalMesh|GetAnimInstance (Variables|Character|GetMesh))))
      (Variables|/Game/Monsters/demon/blueprints/demonABP.demonABP_C|Setalive _asdemon_abp false)
      (Utilities|FlowControl|Delay 2.0)
      (Actor|DestroyActor)
      (CallFunction|Puntuar))))

(event EventBeginPlay
  ;[1 1 1] atacar cada x segundos
  (Utilities|Time|SetTimerbyFunctionName 0 "atacar" 4.0 true)
  (Utilities|FlowControl|Delay 1.2)
  (Utilities|Time|SetTimerbyFunctionName 0 "damage" 4.0 true))

(fn ConstructionScript)

(fn Noperseguir
  (bind _asdemon_abp (Utilities|Casting|CastTodemonABP (Components|SkeletalMesh|GetAnimInstance (Variables|Character|GetMesh))))
  (Variables|/Game/Monsters/demon/blueprints/demonABP.demonABP_C|Setandar _asdemon_abp false))

(fn Damage
  (bind _self self)
  (for _array_element (Collision|GetOverlappingActors (Variables|Default|Getmelee_capsule) "/Game/Characters/assassin/blueprints/asesina.asesina_C" :!class /Script/Engine.PrimitiveComponent)
    (Game|Damage|ApplyDamage _array_element 3e+01 (Pawn|GetController _self) _self)))

(fn Perseguir
  (bind _asdemon_abp (Utilities|Casting|CastTodemonABP (Components|SkeletalMesh|GetAnimInstance (Variables|Character|GetMesh))))
  (Variables|/Game/Monsters/demon/blueprints/demonABP.demonABP_C|Setandar _asdemon_abp true))

(fn Atacar
  (if (Variables|Default|Getcerca)
    (bind _asdemon_abp (Utilities|Casting|CastTodemonABP (Components|SkeletalMesh|GetAnimInstance (Variables|Character|GetMesh))))
    (Variables|/Game/Monsters/demon/blueprints/demonABP.demonABP_C|Setatacar _asdemon_abp true)))

(fn NoAtacar
  (bind _asdemon_abp (Utilities|Casting|CastTodemonABP (Components|SkeletalMesh|GetAnimInstance (Variables|Character|GetMesh))))
  (Variables|/Game/Monsters/demon/blueprints/demonABP.demonABP_C|Setatacar _asdemon_abp false))

(fn Puntuar
  (bind _asasesina (Utilities|Casting|CastToasesina (Game|GetPlayerCharacter 0)))
  (Variables|/Game/Characters/assassin/blueprints/asesina.asesina_C|Setpuntos _asasesina (+ (Variables|/Game/Characters/assassin/blueprints/asesina.asesina_C|Getpuntos _asasesina) 1)))